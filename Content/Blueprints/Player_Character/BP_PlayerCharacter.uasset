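; BP_PlayerCharacter is the player character Blueprint, handling movement, look, jump and a simple ammo count.
; BeginPlay adds the IMC_Playerbase Enhanced Input mapping context, and input actions drive Jump and the Movement and Look functions, with movement relative to control rotation.
; AddAmmo and SubtractAmmo adjust AmmoCount.
; Firing is disconnected: IA_FireGun does nothing, and the FireFirearm logic that fires a child-actor Bp_Firearm and spends ammo never runs.
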(event Input|EnhancedActionEvents|EnhancedInputActionIA_Jump
  (params (ActionValue :type Boolean) (ElapsedSeconds :type Float%20%28double-precision%29) (TriggeredSeconds :type Float%20%28double-precision%29) (InputAction :type Input%20Action%20Object%20Reference :default "/Game/Blueprints/Player_Character/IMC/IA_Jump.IA_Jump"))
  ;[0.2264 1 0.4478 1 40] Movement
  ;;[0.2264 1 0.4478] IA_Jump
  (:Triggered
    (Character|Jump))
  (:Completed
    (Character|StopJumping)))

(event Input|EnhancedActionEvents|EnhancedInputActionIA_Look
  (params (ActionValue :type Vector%202D%20Structure) (ElapsedSeconds :type Float%20%28double-precision%29) (TriggeredSeconds :type Float%20%28double-precision%29) (InputAction :type Input%20Action%20Object%20Reference :default "/Game/Blueprints/Player_Character/IMC/IA_Look.IA_Look"))
  ;[0.2264 1 0.4478 1 40] Movement
  ;;[0.2264 1 0.4478] IA _Look
  (Movement|Look (.x ActionValue) (.y ActionValue)))

(event Input|EnhancedActionEvents|EnhancedInputActionIA_Move
  (params (ActionValue :type Vector%202D%20Structure) (ElapsedSeconds :type Float%20%28double-precision%29) (TriggeredSeconds :type Float%20%28double-precision%29) (InputAction :type Input%20Action%20Object%20Reference :default "/Game/Blueprints/Player_Character/IMC/IA_Move.IA_Move"))
  ;[0.2264 1 0.4478 1 40] Movement
  ;;[0.2264 1 0.4478] IA_Move
  (Movement|Movement (.x ActionValue) (.y ActionValue)))

(event Input|EnhancedActionEvents|EnhancedInputActionIA_FireGun
  (params (ActionValue :type Boolean) (ElapsedSeconds :type Float%20%28double-precision%29) (TriggeredSeconds :type Float%20%28double-precision%29) (InputAction :type Input%20Action%20Object%20Reference :default "/Game/Blueprints/Player_Character/IMC/IA_FireGun.IA_FireGun"))
  ;[1 0.1009 0.001151 1 40] Firearm
  ;;[1 0.1009 0.001151] Fire Firearm
)

(event EventBeginPlay
  ;[1 1 1 1 40] Event Begin Play
  ;;[0.2264 1 0.4478] Add IMC to Player Controler
  (Movement|AddPlayerMovement))

(fn ConstructionScript)

(fn AddPlayerMovement
  (bind _returnvalue (Game|GetPlayerController 0))
  (bind _returnvalue_2 (PlayerController|LocalPlayerSubsystems|GetEnhancedInputLocalPlayerSubsystem _returnvalue))
  ;[0.2264 1 0.4478] Adds IMC to player controller to allow for movement through IMC
  (Utilities|IsValid _returnvalue_2
    (:Is%20Valid
      (Input|AddMappingContext _returnvalue_2 "/Game/Blueprints/Player_Character/IMC/IMC_Playerbase.IMC_Playerbase" 0 "(bIgnoreAllPressedKeysUntilRelease=True,bForceImmediately=False,bNotifyUserSettings=False)"))))

(fn Movement
  (params (X%20Input :type Float%20%28single-precision%29) (Y%20Input :type Float%20%28single-precision%29))
  (bind _returnvalue (Pawn|GetControlRotation :!class /Script/Engine.Pawn))
  (Pawn|Input|AddMovementInput (Math|Vector|GetRightVector (Math|Rotator|MakeRotator (.roll _returnvalue) 0.0 (.yaw _returnvalue))) X%20Input false)
  (Pawn|Input|AddMovementInput (Math|Vector|GetForwardVector (Math|Rotator|MakeRotator 0.0 0.0 (.yaw (Pawn|GetControlRotation :!class /Script/Engine.Pawn)))) Y%20Input false))

(fn Look
  (params (X%20input :type Float%20%28single-precision%29) (Y%20Input :type Float%20%28single-precision%29))
  (Pawn|Input|AddControllerYawInput X%20input)
  (Pawn|Input|AddControllerPitchInput Y%20Input))

(fn AddAmmo
  (params (Ammount%20Added :type Integer))
  (Variables|Firearm|SetAmmo%20Count (+ (Variables|Firearm|GetAmmo%20Count) Ammount%20Added)))

(fn SubtractAmmo
  (params (Ammount%20Added :type Integer))
  (Variables|Firearm|SetAmmo%20Count (- (Variables|Firearm|GetAmmo%20Count) Ammount%20Added)))

(fn FireFirearm)